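; Base enemy character Blueprint whose graph handles the death sequence.
; HandleDeath runs a timeline, scaled by DissolveTime, that drives DissolveAmount on the mesh and equipped weapon materials, then destroys both weapon and character.
; In parallel, it async-loads the supplied Niagara system, attaches it to the mesh and tints its particles with the material's DissolveEdgeColor to match the dissolve.
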(event `self.ReceiveBeginPlay`)

(event `self.HandleDeath`
  (params (NiagaraSystemToPlay :type "NiagaraSystem Soft Object Reference (by ref)"))
  (bind _mesh (`self.Mesh`))
  (bind _returnvalue (`PawnCombatComponent.GetCurrentEquippedWeapon` (`self.CombatComponent`)))
  (`self.HandleDeath_Implementation` NiagaraSystemToPlay)
  (`|ExecutionSequence`
    (:`then_0`
      ;[1 1 1] Disolve material
      (`TimelineComponent.SetPlayRate` (`self.Dissolve Timeline`) (/ 1.0 (`self.DissolveTime`)))
      (bind (_direction _dissolvevalue) (`Timeline|Dissolve Timeline`)
        (:`Update`
          (`MeshComponent.SetScalarParameterValueOnMaterials` (`self.Mesh`) "DissolveAmount" _dissolvevalue)
          (`/Engine/EditorBlueprintResources/StandardMacros.IsValid` _returnvalue
            (:`Is Valid`
              (`MeshComponent.SetScalarParameterValueOnMaterials` (`ARPGWeaponBase.WeaponMesh` _returnvalue) "DissolveAmount" _dissolvevalue))))
        (:`Finished`
          (`/Engine/EditorBlueprintResources/StandardMacros.IsValid` _returnvalue
            (:`Is Valid`
              (`self.K2_DestroyActor` _returnvalue))
            (:`Is Not Valid`
              _))
          (`self.K2_DestroyActor`))))
    (:`then_1`
      ;[1 1 1] Niagara system
      (bind _object (`|LoadAsset` NiagaraSystemToPlay)
        (:`Completed`
          (bind _asniagara_system (cast `NiagaraSystem` _object))
          (bind _returnvalue_2 (`NiagaraFunctionLibrary.SpawnSystemAttached` _asniagara_system (`self.Mesh`) "None" (0.0 0.0 0.0) (struct) "KeepRelativeOffset" true))
          (bind _returnvalue_3 (`PrimitiveComponent.CreateDynamicMaterialInstance` _mesh 0 (`PrimitiveComponent.GetMaterial` _mesh 0) "None"))
          (bind _returnvalue_4 (`MaterialInstanceDynamic.K2_GetVectorParameterValue` _returnvalue_3 "DissolveEdgeColor"))
          (`NiagaraComponent.SetNiagaraVariableLinearColor` _returnvalue_2 "DissolveParticleColor" _returnvalue_4))))))

(fn `UserConstructionScript`)