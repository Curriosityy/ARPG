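; Base Gameplay Ability for enemy hit reactions, activated by a gameplay event.
; On activation it optionally turns the owner to face the event's instigator, switches on a material hit effect and plays a random montage, then applies the GE_UnderAttack effect.
; The ability ends when the montage finishes or is interrupted, or after a short delay if none are set, and switches the hit effect off on end.
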(event `self.K2_ActivateAbilityFromEvent`
  (params (EventData :type "GameplayEventData Structure (by ref)"))
  (`|ExecutionSequence`
    (:`then_0`
      ;[1 1 1] Look at attacker
      (if (`self.FaceToAttacker`)
        (`Actor.K2_SetActorRotation` (`self.GetOwningActorFromActorInfo`) (`KismetMathLibrary.FindLookAtRotation` (`Actor.K2_GetActorLocation` (`self.GetOwningActorFromActorInfo`)) (`Actor.K2_GetActorLocation` (`.Instigator` (break `GameplayEventData` EventData)))) false)))
    (:`then_1`
      (`MeshComponent.SetScalarParameterValueOnMaterials` (`self.GetOwningComponentFromActorInfo`) "HitFxSwitch" 1.0)
      ;[1 1 1] Play montage on hit
      (if (> (`KismetArrayLibrary.Array_Length` (`self.Montages to Play`)) 0)
        (`AbilityTask_PlayMontageAndWait.CreatePlayMontageAndWaitProxy` "None" (`KismetArrayLibrary.Array_Random` (`self.Montages to Play`))
          (:`OnCompleted`
            _)
          (:`OnBlendOut`
            _)
          (:`OnInterrupted`
            _)
          (:`OnCancelled`
            _))
        (else
          (`KismetSystemLibrary.Delay` 0.2)))
      (`self.K2_EndAbility`))
    (:`then_2`
      ;[1 1 1] Add underattack state
      (`self.BP_ApplyGameplayEffectToOwner` "/Game/EnemyCharacter/GameplayEffects/GE_UnderAttack.GE_UnderAttack_C"))))

(event `self.K2_OnEndAbility`
  (params (bWasCancelled :type Boolean))
  (`MeshComponent.SetScalarParameterValueOnMaterials` (`self.GetOwningComponentFromActorInfo`) "HitFxSwitch" 0.0))